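; BP_Mage_NPC3 is a modular battlemage NPC whose outfit is assembled from separate skeletal mesh parts such as dresses, hands, hat, hair, bag and straps.
; The construction script makes every part follow the main Mesh through Leader Pose so they animate together.
; It then sets each part's visibility from its own boolean variable, so outfit variants are configured per instance or default.
; The event graph contains no active logic.
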(event `self.ReceiveBeginPlay`)

(fn `UserConstructionScript`
  (`SkinnedMeshComponent.SetLeaderPoseComponent` (`self.SKM_Mage_Dress_4`) (`self.Mesh`) true false)
  (`SkinnedMeshComponent.SetLeaderPoseComponent` (`self.SKM_Mage_Dress_1`) (`self.Mesh`) true false)
  (`SkinnedMeshComponent.SetLeaderPoseComponent` (`self.SKM_Mage_Dress_2`) (`self.Mesh`) true false)
  (`SkinnedMeshComponent.SetLeaderPoseComponent` (`self.SKM_Mage_Hands_1`) (`self.Mesh`) true false)
  (`SkinnedMeshComponent.SetLeaderPoseComponent` (`self.SKM_Mage_Dress_3`) (`self.Mesh`) true false)
  (`SkinnedMeshComponent.SetLeaderPoseComponent` (`self.SKM_Mage_Bag`) (`self.Mesh`) true false)
  (`SkinnedMeshComponent.SetLeaderPoseComponent` (`self.SKM_Mage_Hands_2`) (`self.Mesh`) true false)
  (`SkinnedMeshComponent.SetLeaderPoseComponent` (`self.SKM_Mage_HatBelt`) (`self.Mesh`) true false)
  (`SkinnedMeshComponent.SetLeaderPoseComponent` (`self.SKM_Mage_Straps`) (`self.Mesh`) true false)
  (`SkinnedMeshComponent.SetLeaderPoseComponent` (`self.SKM_Mage_Decor`) (`self.Mesh`) true false)
  (`SkinnedMeshComponent.SetLeaderPoseComponent` (`self.SKM_Mage_Hair`) (`self.Mesh`) true false)
  (`SkinnedMeshComponent.SetLeaderPoseComponent` (`self.SKM_Mage_Hat`) (`self.Mesh`) true false)
  (`|ExecutionSequence`
    (:`then_0`
      (`SceneComponent.SetVisibility` (`self.SKM_Mage_Dress_1`) (`self.Dress1_Visibility`) false))
    (:`then_1`
      (`SceneComponent.SetVisibility` (`self.SKM_Mage_Dress_2`) (`self.Dress2_Visibility`) false))
    (:`then_2`
      (`SceneComponent.SetVisibility` (`self.SKM_Mage_Dress_3`) (`self.Dress3_Visibility`) false))
    (:`then_3`
      (`SceneComponent.SetVisibility` (`self.SKM_Mage_Dress_4`) (`self.Dress4_Visibility`) false))
    (:`then_4`
      (`SceneComponent.SetVisibility` (`self.SKM_Mage_Hands_1`) (`self.Hands1_Visibility`) false))
    (:`then_5`
      (`SceneComponent.SetVisibility` (`self.SKM_Mage_Hands_2`) (`self.Hands2_Visibility`) false))
    (:`then_6`
      (`SceneComponent.SetVisibility` (`self.SKM_Mage_HatBelt`) (`self.HatBelt_Visibility`) false))
    (:`then_7`
      (`SceneComponent.SetVisibility` (`self.SKM_Mage_Straps`) (`self.Straps_Visibility`) false))
    (:`then_8`
      (`SceneComponent.SetVisibility` (`self.SKM_Mage_Decor`) (`self.Decor_Visibility`) false))
    (:`then_9`
      (`SceneComponent.SetVisibility` (`self.SKM_Mage_Bag`) (`self.Bag_Visibility`) false))
    (:`then_10`
      (`SceneComponent.SetVisibility` (`self.SKM_Mage_Hair`) (`self.Hair_Visibility`) false))
    (:`then_11`
      (`SceneComponent.SetVisibility` (`self.SKM_Mage_Hat`) (`self.Hat_Visibility`) false))))